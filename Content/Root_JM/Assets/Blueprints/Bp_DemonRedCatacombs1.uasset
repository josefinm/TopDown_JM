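; Catacombs demon sentry that scans for the player with a detection cone and a spotlight.
; While nothing is detected, a Delay on Tick steps the demon's yaw every two seconds, with nested FlipFlops producing a back-and-forth sweep across a quarter turn.
; Cone overlaps with the player character set DETECTED, which halts the sweep, turn the spotlight red or back to green, and print debug messages.
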(event OnComponentBeginOverlap(Cone)
  (params (OverlappedComponent :type Primitive%20Component%20Object%20Reference) (OtherActor :type Actor%20Object%20Reference) (OtherComp :type Primitive%20Component%20Object%20Reference) (OtherBodyIndex :type Integer) (bFromSweep :type Boolean) (SweepResult :type Hit%20Result%20Structure%20%28by%20ref%29))
  ;[1 1 1] Identifying Player
  (Utilities|Casting|CastToCorePlayerCharacter OtherActor)
  (Development|PrintString "DETECTED!" true true "(R=1.000000,G=0.006920,B=0.000000,A=1.000000)")
  (Rendering|Components|Light|SetLightColor (Variables|Default|GetSpotLight) "(R=1.000000,G=0.000000,B=0.000000,A=1.000000)" true)
  (Variables|Default|SetdETECTED true))

(event OnComponentEndOverlap(Cone)
  (params (OverlappedComponent :type Primitive%20Component%20Object%20Reference) (OtherActor :type Actor%20Object%20Reference) (OtherComp :type Primitive%20Component%20Object%20Reference) (OtherBodyIndex :type Integer))
  ;[1 1 1] Identifying Player
  (Utilities|Casting|CastToCorePlayerCharacter OtherActor)
  (Development|PrintString "Gone!" true true "(R=0.000000,G=0.331652,B=1.000000,A=1.000000)")
  (Rendering|Components|Light|SetLightColor (Variables|Default|GetSpotLight) "(R=0.000000,G=1.000000,B=0.082283,A=1.000000)" true)
  (Variables|Default|SetdETECTED false))

(event EventTick
  (params (DeltaSeconds :type Float%20%28single-precision%29))
  (Utilities|FlowControl|Delay 2.0)
  (if (not (Variables|Default|GetdETECTED))
    (Utilities|FlowControl|FlipFlop
      (:A
        (Utilities|FlowControl|FlipFlop
          (:A
            (Variables|Default|SetRotation 45.0))
          (:B
            (Variables|Default|SetRotation 45.0))))
      (:B
        (Utilities|FlowControl|FlipFlop
          (:A
            (Variables|Default|SetRotation 9e+01))
          (:B
            (Variables|Default|SetRotation 0.0)))))
    (Transformation|SetRelativeRotation (Variables|Default|GetDemon) (Math|Rotator|MakeRotator 0.0 0.0 (Variables|Default|GetRotation)) false false)))

(fn ConstructionScript)