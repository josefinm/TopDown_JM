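; BP_Gargoyle is a patrolling detector whose Gargoyle component loops along a spline until it spots the player.
; Tick advances the spline distance at a constant rate, resets it at the end, and updates only the relative location.
; Collision overlaps with CorePlayerCharacter set Detected, pausing movement and turning the spotlight red with a debug print.
; Ending the overlap turns the light green and resumes the patrol.
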(event OnComponentBeginOverlap(Collision)
  (params (OverlappedComponent :type Primitive%20Component%20Object%20Reference) (OtherActor :type Actor%20Object%20Reference) (OtherComp :type Primitive%20Component%20Object%20Reference) (OtherBodyIndex :type Integer) (bFromSweep :type Boolean) (SweepResult :type Hit%20Result%20Structure%20%28by%20ref%29))
  ;[1 1 1] Identifying Player
  (Utilities|Casting|CastToCorePlayerCharacter OtherActor)
  (Development|PrintString "DETECTED!" true true "(R=1.000000,G=0.006920,B=0.000000,A=1.000000)")
  (Rendering|Components|Light|SetLightColor (Variables|Default|GetSpotLight) "(R=1.000000,G=0.000000,B=0.000000,A=1.000000)" true)
  (Variables|Default|SetDetected true))

(event OnComponentEndOverlap(Collision)
  (params (OverlappedComponent :type Primitive%20Component%20Object%20Reference) (OtherActor :type Actor%20Object%20Reference) (OtherComp :type Primitive%20Component%20Object%20Reference) (OtherBodyIndex :type Integer))
  ;[1 1 1] Identifying Player
  (Utilities|Casting|CastToCorePlayerCharacter OtherActor)
  (Development|PrintString "Gone!" true true "(R=0.000000,G=0.331652,B=1.000000,A=1.000000)")
  (Rendering|Components|Light|SetLightColor (Variables|Default|GetSpotLight) "(R=0.000000,G=1.000000,B=0.082283,A=1.000000)" true)
  (Variables|Default|SetDetected false))

(event EventTick
  (params (DeltaSeconds :type Float%20%28single-precision%29))
  (bind _spline (Variables|Default|GetSpline))
  (bind _returnvalue (Spline|GetSplineLength _spline))
  ;[1 1 1] Rotating on Spline
  (if (not (Variables|Default|GetDetected))
    (if (>= (Variables|Default|GetCurrentDistanceAlongSpline) _returnvalue)
      (Variables|Default|SetCurrentDistanceAlongSpline 0.0)
      (else
        (bind _output_get (Variables|Default|SetCurrentDistanceAlongSpline (Math|Interpolation|FInterptoConstant (Variables|Default|GetCurrentDistanceAlongSpline) _returnvalue DeltaSeconds (Variables|Default|GetGargoyleRotatingSpeed))))
        (Transformation|SetRelativeLocation (Variables|Default|GetGargoyle) (Spline|GetLocationatDistanceAlongSpline (Variables|Default|GetSpline) _output_get "Local") false false)))))

(fn ConstructionScript)