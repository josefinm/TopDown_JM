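; BP_Balcony is a Blueprint that shows or hides balcony and broken-floor components based on where the player goes.
; Balconies and FloorBroken are hidden in game on BeginPlay.
; Overlapping TriggerUpp with a CorePlayerCharacter reveals both components, and overlapping TriggerNer hides them again.
; Visibility changes do not propagate to child components.
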(event OnComponentBeginOverlap(TriggerUpp)
  (params (OverlappedComponent :type Primitive%20Component%20Object%20Reference) (OtherActor :type Actor%20Object%20Reference) (OtherComp :type Primitive%20Component%20Object%20Reference) (OtherBodyIndex :type Integer) (bFromSweep :type Boolean) (SweepResult :type Hit%20Result%20Structure%20%28by%20ref%29))
  (Utilities|Casting|CastToCorePlayerCharacter OtherActor)
  (Development|SetHiddeninGame (Variables|Default|GetBalconies) false false))

(event OnComponentBeginOverlap(TriggerNer)
  (params (OverlappedComponent :type Primitive%20Component%20Object%20Reference) (OtherActor :type Actor%20Object%20Reference) (OtherComp :type Primitive%20Component%20Object%20Reference) (OtherBodyIndex :type Integer) (bFromSweep :type Boolean) (SweepResult :type Hit%20Result%20Structure%20%28by%20ref%29))
  (Utilities|Casting|CastToCorePlayerCharacter OtherActor)
  (Development|SetHiddeninGame (Variables|Default|GetBalconies) true false))

(event EventBeginPlay
  (Development|SetHiddeninGame (Variables|Default|GetBalconies) true false))

(fn ConstructionScript)