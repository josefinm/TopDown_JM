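; Demon gargoyle sentry that sweeps its gaze back and forth and freezes while the player is inside its detection cone.
; Tick uses a one-second Delay to advance a counter, which RotateGargoyle maps to fixed yaw steps on the Demon component.
; Cone overlaps with CorePlayerCharacter set DETECTED, halting the counter, switch the SpotLight between red and green, and print debug messages.
; A nested FlipFlop chain is left unconnected.
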(event OnComponentBeginOverlap(Cone)
  (params (OverlappedComponent :type Primitive%20Component%20Object%20Reference) (OtherActor :type Actor%20Object%20Reference) (OtherComp :type Primitive%20Component%20Object%20Reference) (OtherBodyIndex :type Integer) (bFromSweep :type Boolean) (SweepResult :type Hit%20Result%20Structure%20%28by%20ref%29))
  ;[1 1 1] Identifying Player
  (Utilities|Casting|CastToCorePlayerCharacter OtherActor)
  (Development|PrintString "DETECTED!" true true "(R=1.000000,G=0.006920,B=0.000000,A=1.000000)")
  (Rendering|Components|Light|SetLightColor (Variables|Default|GetSpotLight) "(R=1.000000,G=0.000000,B=0.000000,A=1.000000)" true)
  (Variables|Default|SetdETECTED true))

(event OnComponentEndOverlap(Cone)
  (params (OverlappedComponent :type Primitive%20Component%20Object%20Reference) (OtherActor :type Actor%20Object%20Reference) (OtherComp :type Primitive%20Component%20Object%20Reference) (OtherBodyIndex :type Integer))
  ;[1 1 1] Identifying Player
  (Utilities|Casting|CastToCorePlayerCharacter OtherActor)
  (Development|PrintString "Gone!" true true "(R=0.000000,G=0.331652,B=1.000000,A=1.000000)")
  (Rendering|Components|Light|SetLightColor (Variables|Default|GetSpotLight) "(R=0.000000,G=1.000000,B=0.082283,A=1.000000)" true)
  (Variables|Default|SetdETECTED false))

(event Custom|RotateGargoyle
  (if (== (Variables|Default|GetCount) 1)
    (Variables|Default|SetRotation 4e+01)
    (Transformation|SetRelativeRotation (Variables|Default|GetDemon) (Math|Rotator|MakeRotator 0.0 0.0 (Variables|Default|GetRotation)) false false :!label _label)
    (elif (== (Variables|Default|GetCount) 2)
      (Variables|Default|SetRotation 7e+01)
      (goto _label)
      (elif (== (Variables|Default|GetCount) 3)
        (Variables|Default|SetRotation 9e+01)
        (goto _label)
        (elif (== (Variables|Default|GetCount) 4)
          (Variables|Default|SetRotation 7e+01)
          (goto _label)
          (elif (== (Variables|Default|GetCount) 5)
            (Variables|Default|SetRotation 4e+01)
            (goto _label)
            (elif (== (Variables|Default|GetCount) 0)
              (Variables|Default|SetRotation 0.0)
              (goto _label)
              (else
                (Development|PrintString "Wrong")))))))))

(event EventTick
  (params (DeltaSeconds :type Float%20%28single-precision%29))
  (Utilities|FlowControl|Sequence
    (:then_0
      (Utilities|FlowControl|Delay 1.0)
      (if (not (Variables|Default|GetdETECTED))
        (if (>= (Variables|Default|GetCount) 5)
          (Variables|Default|SetCount 0)
          (else
            (Variables|Default|SetCount (+ (Variables|Default|GetCount) 1))))))
    (:then_1
      (CallFunction|RotateGargoyle))))

(fn ConstructionScript)