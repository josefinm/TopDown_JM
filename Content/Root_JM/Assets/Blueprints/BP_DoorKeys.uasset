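; BP_DoorKeys is a door that opens for a player carrying both priest keys.
; When its trigger volume overlaps a CorePlayerCharacter, it checks that both HasKey1 and HasKey2 are set.
; If so, a timeline slides the Door component from Begin to End by lerping its relative location; otherwise it prints a message that both keys are required.
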(event OnComponentBeginOverlap(Trigger)
  (params (OverlappedComponent :type Primitive%20Component%20Object%20Reference) (OtherActor :type Actor%20Object%20Reference) (OtherComp :type Primitive%20Component%20Object%20Reference) (OtherBodyIndex :type Integer) (bFromSweep :type Boolean) (SweepResult :type Hit%20Result%20Structure%20%28by%20ref%29))
  (bind _ascore_player_character (Utilities|Casting|CastToCorePlayerCharacter OtherActor))
  (if (and (Variables|/Game/Root_JM/Core/Framework/CorePlayerCharacter.CorePlayerCharacter_C|GethasKey1 _ascore_player_character) (Variables|/Game/Root_JM/Core/Framework/CorePlayerCharacter.CorePlayerCharacter_C|GethasKey2 _ascore_player_character))
    (bind _newtrack_0 (Timeline|Timeline_0 Play)
      (:Update
        (Transformation|SetRelativeLocation (Variables|Default|GetDoor) (Math|Vector|Lerp(Vector) (Variables|Default|GetBegin) (Variables|Default|GetEnd) _newtrack_0) false false)))
    (else
      (Development|PrintString "Requires both PREIST KEYS"))))

(fn ConstructionScript)